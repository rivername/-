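; Player character Blueprint that can flip gravity, turning upside down to walk on ceilings.
; Each Tick sets gravity scale and jump velocity from the Gravity flag; when it toggles, the character starts falling and a timeline drives its roll.
; While inverted, vertical line traces substitute for floor detection, switching between Walking and Falling, with a MobiusObject hit on the head side forcing Walking.
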(event EventBeginPlay
  ;[1 1 1] 初期化
  (Variables|Default|Settmp_G (not (Variables|Default|GetGravity))))

(event EventTick
  (params (DeltaSeconds :type Float%20%28single-precision%29))
  ;[1 1 1] 反転時の接地判定
  (CallFunction|ReverceWalking)
  ;[1 1 1] キャラクターの反転
  (CallFunction|CharacterReverseRotation)
  ;[1 1 1] 重力切り替え
  (CallFunction|GravityChange)
  (if (Math|Boolean|Equal(Boolean) (Variables|Default|GetGravity) (Variables|Default|Gettmp_G))
    (Variables|Default|Settmp_G (not (Variables|Default|GetGravity)))
    (Pawn|Components|CharacterMovement|SetMovementMode (Variables|Character|GetCharacterMovement) "MOVE_Falling" 0)
    (if (Variables|Default|GetGravity)
      (bind _rotasion_x (Timeline|Rotation%20Rate Reverse)
        (:Update
          (Variables|Default|SetReverse%20X _rotasion_x)
          (CallFunction|CharacterReverseRotation))
        (:Finished
          (Variables|Default|SetNow%20Rotation false)))
      (else
        (Timeline|Rotation%20Rate Play)))))

(fn ConstructionScript)

(fn CharacterReverseRotation
  (bind _returnvalue (Transformation|GetActorRotation))
  ;[1 1 1] キャラの上下反転
  (Transformation|SetActorRotation (Math|Rotator|MakeRotator (Variables|Default|GetReverse%20X) (.pitch _returnvalue) (.yaw _returnvalue)))
  (if (AI|Components|NavMovement|IsMovingonGround (Variables|Character|GetCharacterMovement))
    (Variables|Default|SetJumping false))
  (if (AI|Components|NavMovement|IsFalling (Variables|Character|GetCharacterMovement))
    (Variables|Default|Setis%20Falling true)
    (else
      (Variables|Default|Setis%20Falling false))))

(fn GravityChange
  ;[1 1 1] 重力切り替え
  (Variables|Default|SetNow%20Rotation true)
  (if (Variables|Default|GetGravity)
    (Variables|/Script/Engine.CharacterMovementComponent|SetGravityScale (Variables|Character|GetCharacterMovement) 1.0)
    (Variables|Default|SetJump%20vel 6e+02)
    (else
      (Variables|/Script/Engine.CharacterMovementComponent|SetGravityScale (Variables|Character|GetCharacterMovement) -1.0)
      (Variables|Default|SetJump%20vel -6e+02))))

(fn ReverceWalking
  (bind _returnvalue (Transformation|GetActorLocation))
  (bind _returnvalue_2 (Transformation|GetActorLocation))
  (bind _returnvalue_3 (Transformation|GetActorLocation))
  ;[1 1 1] 反転時のみ
  (if (not (Variables|Default|GetGravity))
    ;[1 1 1] 足元から床の判定
    (bind _returnvalue_4 (Collision|LineTraceForObjects (+ _returnvalue "0, 0,50.000000") (+ _returnvalue "0.000000,0.000000,97.000000") (Utilities|Array|MakeArray "ObjectTypeQuery1" "ObjectTypeQuery2") false 0 "ForOneFrame"))
    (if _returnvalue_4
      (Pawn|Components|CharacterMovement|SetMovementMode (Variables|Character|GetCharacterMovement) "MOVE_Walking" 0))
    ;[1 1 1] 頭から天井の判定
    (bind _returnvalue_5 (Collision|LineTraceForObjects (+ _returnvalue_2 "0, 0,-50.000000") (+ _returnvalue_2 "0.000000,0.000000,-100.000000") (Utilities|Array|MakeArray "ObjectTypeQuery1" "ObjectTypeQuery2") false 0 "ForOneFrame"))
    (if _returnvalue_5
      (Pawn|Components|CharacterMovement|SetMovementMode (Variables|Character|GetCharacterMovement) "MOVE_Falling" 0))
    ;[1 1 1] Mobius_obujectが降ってきた場合
    (bind (_outhit _returnvalue_6) (Collision|LineTraceForObjects (+ _returnvalue_3 "0, 0,-50.000000") (+ _returnvalue_3 "0.000000,0.000000,-100.000000") (Utilities|Array|MakeArray "ObjectTypeQuery1" "ObjectTypeQuery2") false 0 "ForOneFrame"))
    (if _returnvalue_6
      (Utilities|Casting|CastTo00_MobiusObject_BP (.HitActor (Collision|BreakHitResult _outhit)))
      (Pawn|Components|CharacterMovement|SetMovementMode (Variables|Character|GetCharacterMovement) "MOVE_Walking" 0))))

(fn CharaDebugStatus
  (bind _returnvalue (Utilities|Time|GetWorldDeltaSeconds))
  (bind _charactermovement (Variables|Character|GetCharacterMovement))
  (if (Pawn|Components|CharacterMovement|IsWalking _charactermovement)
    (Development|PrintString "wallking" true true "(R=0.000000,G=0.660000,B=1.000000,A=1.000000)" _returnvalue))
  (if (AI|Components|NavMovement|IsMovingonGround _charactermovement)
    (Development|PrintString "Move Ground" true true "(R=0.000000,G=0.660000,B=1.000000,A=1.000000)" _returnvalue))
  (if (AI|Components|NavMovement|IsFalling _charactermovement)
    (Development|PrintString "Falling" true true "(R=0.000000,G=0.660000,B=1.000000,A=1.000000)" _returnvalue))
  (if (Variables|Default|GetJumping)
    (Development|PrintString "Jump true" true true "(R=0.000000,G=0.660000,B=1.000000,A=1.000000)" _returnvalue)
    (else
      (Development|PrintString "Jump false" true true "(R=0.000000,G=0.660000,B=1.000000,A=1.000000)" _returnvalue)))
  (if true
    _
    (else
      _))
  (Development|PrintString (Utilities|String|ToString(Float) (Variables|Default|GetJump%20vel)) true true "(R=0.000000,G=0.660000,B=1.000000,A=1.000000)" _returnvalue))