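; Shutter actor that slides vertically open or closed through timelines driven by OpenAndClose, which SetOpen and ToggleOpen events change.
; Non-main shutters copy that flag from their attached parent Shutter_BP each tick, so attached shutters move together.
; Tick also ANDs the pressed state of its pressure plates into AndSwitch, which on the main shutter only gates one-shot open and close sounds, not movement.
; SoundPlay is an empty stub.
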(event Custom|Toggle%20Open
  (Variables|Default|SetOpen%20and%20Close (not (Variables|Default|GetOpen%20and%20Close))))

(event Custom|Set%20Open
  (params (Set%20Open :type Boolean))
  (bind _output_get (Variables|Default|SetOpen%20and%20Close Set%20Open))
  (if _output_get
    _))

(event Custom|Tick
  (bind _returnvalue (Transformation|GetActorLocation))
  (if (Variables|Default|GetIs%20Main?)
    (if (Variables|Default|GetAnd%20Switch)
      (Utilities|FlowControl|DoOnce false :!label _label
        (:Completed
          (Variables|Default|SetOpenShutter true)
          (Audio|PlaySoundatLocation "/Game/18_Kawana/BGM/Shutter.Shutter" _returnvalue "0, 0, 0" 1.0 1.0 0.0 "/Game/17_Kawasaki/Sound/SA_SoundEffect.SA_SoundEffect" 0 0)
          (goto _label_2 Reset)))
      (elif (Variables|Default|GetOpenShutter)
        (Utilities|FlowControl|DoOnce false :!label _label_2
          (:Completed
            (Variables|Default|SetOpenShutter false)
            (Development|PrintString "Hello")
            (Audio|PlaySoundatLocation "/Game/18_Kawana/BGM/Shutter.Shutter" _returnvalue "0, 0, 0" 1.0 1.0 0.0 "/Game/17_Kawasaki/Sound/SA_SoundEffect.SA_SoundEffect" 0 0)
            (goto _label Reset)))))))

(event EventTick
  (params (DeltaSeconds :type Float%20%28single-precision%29))
  (CallFunction|Tick)
  (bind _and_switch (CallFunction|GetandSwitchState))
  (Variables|Default|SetAnd%20Switch _and_switch)
  (CallFunction|SyncwithParent)
  (CallFunction|SoundPlay)
  ;[1 1 1] Mode Always
  (if (Variables|Default|GetOpen%20and%20Close)
    (bind _open (Timeline|Open%20Close1 Play)
      (:Update
        (Transformation|SetRelativeLocation (Variables|Default|Getshutter) (Math|Vector|MakeVector 0.0 0.0 _open) false false)
        ;[1 1 1] Mode switching
        (if (Variables|Default|GetOpen%20and%20Close)
          (bind _open_2 (Timeline|Open%20Close2 Play)
            (:Update
              (Transformation|SetRelativeLocation (Variables|Default|Getshutter) (Math|Vector|MakeVector 0.0 0.0 _open_2) false false)))
          (else
            (Timeline|Open%20Close2 Reverse)))))
    (else
      (Timeline|Open%20Close1 Reverse))))

(fn ConstructionScript)

(fn SyncwithParent
  ;[1 1 1] 同期
  (if (not (Variables|Default|GetIs%20Main?))
    (bind _asshutter_bp (Utilities|Casting|CastToShutter_BP (Actor|GetAttachParentActor)))
    (Variables|Default|SetOpen%20and%20Close (Variables|Shutter_BP_C|GetOpen%20and%20Close _asshutter_bp))))

(fn SoundPlay)

(fn GetandSwitchState
  (for _array_element (Variables|Default|GetPressure%20Plate%20Arry)
    (if (not (Variables|/Game/17_Kawasaki/BP/PressurePlate/PressurePlate_BP.PressurePlate_BP_C|GetIs%20Pressed? _array_element))
      (LocalVariables|SetTmp false)))
  (return (LocalVariables|GetTmp)))