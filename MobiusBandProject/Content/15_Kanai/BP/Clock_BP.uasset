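; Wall-clock Blueprint that shows the current system time by rolling separate hour, minute and second hand meshes every Tick.
; Hand angles come from Now(), with hour and minute hands advancing fractionally between marks.
; When the second-hand angle changes, it plays a 2D tick sound if PlaySound is enabled and MobiusGameInstance's current room matches its RoomClass.
; A FirstSound flag suppresses the initial tick.
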(event EventTick
  (params (DeltaSeconds :type Float%20%28single-precision%29))
  (bind _angle (CallFunction|GetHourHandAngle))
  (Transformation|SetRelativeRotation (Variables|Default|GetSM_HourHand) (Math|Rotator|MakeRotator _angle 0.0 0.0) false false)
  (bind _angle_2 (CallFunction|GetMinuteHandAngle))
  (Transformation|SetRelativeRotation (Variables|Default|GetSM_MinuteHand) (Math|Rotator|MakeRotator _angle_2 0.0 0.0) false false)
  (bind _angle_3 (CallFunction|GetSecondHandAngle))
  (if (== _angle_3 (Variables|Default|GetCurrentRoll%20of%20SecondHand))
    _
    (else
      (CallFunction|PlaySoundClock)))
  (bind _output_get (Variables|Default|SetCurrentRoll%20of%20SecondHand _angle_3))
  (Transformation|SetRelativeRotation (Variables|Default|GetSM_SecondHand) (Math|Rotator|MakeRotator _output_get 0.0 0.0) false false))

(fn ConstructionScript)

(fn GetHourHandAngle
  (bind _returnvalue (Math|DateTime|Now))
  (return (+ (* (Class|KismetMathLibrary|GetHour12 _returnvalue) (/ 3.6e+02 12.0)) (* (Class|KismetMathLibrary|GetMinute _returnvalue) (/ 3.6e+02 7.2e+02)))))

(fn GetMinuteHandAngle
  (bind _returnvalue (Math|DateTime|Now))
  (return (+ (* (Class|KismetMathLibrary|GetMinute _returnvalue) (/ 3.6e+02 6e+01)) (* (Class|KismetMathLibrary|GetSecond _returnvalue) (/ 3.6e+02 3.6e+03)))))

(fn GetSecondHandAngle
  (return (* (Class|KismetMathLibrary|GetSecond (Math|DateTime|Now)) (/ 3.6e+02 6e+01))))

(fn PlaySoundClock
  (bind _asmobius_game_instance (Utilities|Casting|CastToMobiusGameInstance (Game|GetGameInstance)))
  (bind _mobiusroomclass (Default|GetCurrentRoomClass _asmobius_game_instance))
  (if (Math|Boolean|ANDBoolean (== _mobiusroomclass (Variables|Default|GetRoomClass)) (Variables|Default|GetbPlaySound) (not (Variables|Default|GetbFirstSound))) ; プレイヤーと同じ部屋にいて、再生許可された
    (Audio|PlaySound2D "/Game/15_Kanai/Sounds/Clock_wav.Clock_wav" 1.0 1.0 0.0 0 0)
    (else
      (Variables|Default|SetbFirstSound false))))