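; Actor that plays a scrolling credits roll driven by the Credit data table.
; StartScroll reads rows by incrementing index, spawns one of four widget classes chosen by the row's Type, and starts its movement with name, speed and font size.
; A timer schedules the next row using its interval scaled by scroll speed.
; Each widget's MoveEnd event removes the oldest widget; a missing row ends the roll.
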(event Custom|StartScroll
  (bind _returnvalue (Utilities|GetDataTableRow "/Game/15_Kanai/HUD/Credit.Credit" (Utilities|String|StringToName (Utilities|String|ToString(Integer) (Variables|Default|Getindex))))
    (:then
      (bind _returnvalue_2 (UserInterface|CreateWidget (Utilities|Array|Get(acopy) (Variables|Default|GetCreditArray) (.Type (Utilities|Struct|BreakS_Credit _returnvalue)))))
      (Utilities|Array|Add (Variables|Default|GetCreaditWidget) _returnvalue_2)
      (UserInterface|Viewport|AddtoViewport _returnvalue_2 0)
      (Class|BPIStartMove|StartMove(Message) _returnvalue_2 (.Name (Utilities|Struct|BreakS_Credit _returnvalue)) (Variables|Default|GetScrollSpeed) (.fontsize (Utilities|Struct|BreakS_Credit _returnvalue)))
      (switch int (.Type (Utilities|Struct|BreakS_Credit _returnvalue))
        (:0
          (bind _aswidget_00 (Utilities|Casting|CastToWidget00 _returnvalue_2))
          (EventDispatchers|BindEventtoMoveEnd _aswidget_00 (delegate Custom|RemoveWidget)))
        (:1
          (bind _aswidget_01 (Utilities|Casting|CastToWidget01 _returnvalue_2))
          (EventDispatchers|BindEventtoMoveEnd _aswidget_01 (delegate Custom|RemoveWidget)))
        (:2
          (bind _aswidget_02 (Utilities|Casting|CastToWidget02 _returnvalue_2))
          (EventDispatchers|BindEventtoMoveEnd _aswidget_02 (delegate Custom|RemoveWidget)))
        (:3
          (bind _aswidget_03 (Utilities|Casting|CastToWidget03 _returnvalue_2))
          (EventDispatchers|BindEventtoMoveEnd _aswidget_03 (delegate Custom|RemoveWidget))))
      (Utilities|Time|SetTimerbyEvent (delegate Custom|StartScroll) (/ (.Interval (Utilities|Struct|BreakS_Credit _returnvalue)) (Variables|Default|GetScrollSpeed)))
      (Variables|Default|Setindex (+ (Variables|Default|Getindex) 1)))
    (:RowNotFound
      (Development|PrintString "Hello"))))

(event Custom|RemoveWidget
  (bind _creaditwidget (Variables|Default|GetCreaditWidget))
  (Widget|RemovefromParent (Utilities|Array|Get(acopy) _creaditwidget))
  (Utilities|Array|RemoveIndex _creaditwidget))

(event EventBeginPlay
  (Variables|Default|SetCreditArray (Utilities|Array|MakeArray "/Game/15_Kanai/HUD/Widget00.Widget00_C" "/Game/15_Kanai/HUD/Widget01.Widget01_C" "/Game/15_Kanai/HUD/Widget02.Widget02_C" "/Game/15_Kanai/HUD/Widget03.Widget03_C"))
  (Variables|Default|SetScrollSpeed 2.0)
  (CallFunction|StartScroll))

(fn ConstructionScript)