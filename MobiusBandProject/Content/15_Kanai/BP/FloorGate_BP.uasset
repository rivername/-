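; FloorGate_BP is a floor gate whose left and right sides slide apart along local Y, each by up to CellSize.
; A SetOpen flag, set externally or flipped by ToggleOpen, is polled every Tick to play or reverse the Open timeline that moves both sides.
; ToggleOpen is gated by a DoOnce until ResetToggleOpenDoOnce is called.
; OpenStart opens the gate at BeginPlay, and construction clears it for non-Toggleable gates.
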(event Custom|Toggle%20Open
  ;[1 1 1] 外部呼出し関数
  (Utilities|FlowControl|DoOnce false
    (:Completed
      (Variables|Default|SetSet%20Open? (not (Variables|Default|GetSet%20Open?))))))

(event Custom|Set%20Open
  (params (open :type Boolean))
  ;[1 1 1] 外部呼出し関数
  (Variables|Default|SetSet%20Open? open))

(event Custom|Event%20Reset%20ToggleOpen%20DoOnce
  ;[1 1 1] 外部呼出し関数
  (Utilities|FlowControl|DoOnce false) ; enters at Reset
)

(event EventTick
  (params (DeltaSeconds :type Float%20%28single-precision%29))
  ;[1 1 1] イベント
  (if (Variables|Default|GetSet%20Open?)
    (bind _0_1 (Timeline|open Play)
      (:Update
        (CallFunction|OpenLeft _0_1)
        (CallFunction|OpenRight _0_1)))
    (else
      (Timeline|open Reverse))))

(event EventBeginPlay
  ;[1 1 1] イベント
  (|CallParentFunction)
  (if (Variables|Default|GetbOpenStart)
    (Variables|Default|SetSet%20Open? true)))

(fn ConstructionScript
  (|CallParentFunction)
  (Variables|Default|SetInit%20Location%20L (.location (Transformation|GetRelativeTransform (Variables|Default|GetLeft%20side))))
  (Variables|Default|SetInit%20Location%20R (.location (Transformation|GetRelativeTransform (Variables|Default|GetRight%20side))))
  (if (not (Variables|Default|GetbToggleable))
    (Variables|Default|SetbOpenStart false)))

(fn OpenLeft
  (params (α :type Float%20%28single-precision%29))
  (Transformation|SetRelativeLocation (Variables|Default|GetLeft%20side) (Math|Vector|MakeVector 0.0 (- (.y (Variables|Default|GetInit%20Location%20L)) (* α (Variables|Default|GetCellSize))) 0.0) false false))

(fn OpenRight
  (params (α :type Float%20%28single-precision%29))
  (Transformation|SetRelativeLocation (Variables|Default|GetRight%20side) (Math|Vector|MakeVector 0.0 (+ (.y (Variables|Default|GetInit%20Location%20R)) (* α (Variables|Default|GetCellSize))) 0.0) false false))