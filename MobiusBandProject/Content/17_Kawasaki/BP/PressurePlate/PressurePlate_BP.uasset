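; Pressure plate for the Mobius stages that sinks under the player or Mobius objects and fires configurable pressed and released actions.
; While enabled in the current stage, Tick box-traces above the plate to set the pressed state and play sounds.
; The main plate's timeline moves the mesh, then drives key boxes, shutters, floor gates or stage clearing.
; Non-main plates copy their height from an attached parent plate.
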(event Custom|Event%20Hit
  (if (or (Variables|Default|GetPlayerTriggered) (Variables|Default|GetObjectTriggered))
    (Variables|Default|SetIs%20Pressed? true)
    (else
      (Variables|Default|SetIs%20Pressed? false))))

(event Custom|Press%20And%20Release
  (if (Variables|Default|GetIs%20Main?)
    (if (Variables|Default|GetIs%20Pressed?)
      (bind _plate_location_z (Timeline|PressurePlate%20Timeline Play)
        (:Update
          (bind _output_get (Variables|Default|SetRelative%20Location%20Z _plate_location_z))
          (Transformation|SetRelativeLocation (Variables|Default|GetPlate%20Mesh) (Math|Vector|MakeVector 0.0 0.0 _output_get) false false))
        (:Finished
          (if (Variables|Default|GetIs%20Pressed?)
            (Variables|Default|SetCurrentActions (Variables|Default|GetPressedActions))
            (for _array_element (Variables|Default|GetCurrentActions) :!label _label
              (if (Utilities|Enum|Equal(Enum) _array_element "NewEnumerator0")
                (for _array_element_2 (Variables|Default|GetKeyBoxes)
                  (Default|SetOpenState _array_element_2 true))
                (elif (Utilities|Enum|Equal(Enum) _array_element "NewEnumerator2")
                  (for _array_element_3 (Variables|Default|GetKeyBoxes)
                    (Default|SetOpenState _array_element_3 false))
                  (elif (Utilities|Enum|Equal(Enum) _array_element "NewEnumerator1")
                    (Utilities|FlowControl|DoOnce false :!label _label_2
                      (:Completed
                        (for _array_element_4 (Variables|Default|GetShutteres)
                          (Default|SetOpen _array_element_4 true))))
                    (elif (Utilities|Enum|Equal(Enum) _array_element "NewEnumerator3")
                      (for _array_element_5 (Variables|Default|GetShutteres)
                        (Default|SetOpen _array_element_5 false)
                        (goto _label_2 Reset))
                      (elif (Utilities|Enum|Equal(Enum) _array_element "NewEnumerator4")
                        (Utilities|FlowControl|DoOnce true
                          (:Completed
                            (for _array_element_6 (Variables|Default|GetShutteres)
                              (Default|ToggleOpen _array_element_6))))
                        (elif (Utilities|Enum|Equal(Enum) _array_element "NewEnumerator5")
                          (Utilities|FlowControl|DoOnce true :!label _label_3
                            (:Completed
                              (bind _asmobius_character (Utilities|Casting|CastTo (Game|GetPlayerCharacter 0)))
                              (Variables|Default|SetStageCleared _asmobius_character true)))
                          (elif (Utilities|Enum|Equal(Enum) _array_element "NewEnumerator6")
                            (bind _returnvalue (Actor|GetActorOfClass "/Game/99_MyContents/BP/ParentClasses/MobiusRoom.MobiusRoom_C"))
                            (Default|EventDiscardStageCleared _returnvalue)
                            (goto _label_3 Reset)
                            (elif (Utilities|Enum|Equal(Enum) _array_element "NewEnumerator7")
                              (for _array_element_7 (Variables|Default|GetFloorGates)
                                (Default|SetOpen _array_element_7 true))
                              (elif (Utilities|Enum|Equal(Enum) _array_element "NewEnumerator8")
                                (for _array_element_8 (Variables|Default|GetFloorGates)
                                  (Default|SetOpen _array_element_8 false))
                                (elif (Utilities|Enum|Equal(Enum) _array_element "NewEnumerator9")
                                  (for _array_element_9 (Variables|Default|GetFloorGates)
                                    (Default|ToggleOpen _array_element_9)))))))))))))
            (elif (Variables|Default|GetIs%20Moving?)
              (Variables|Default|SetIs%20Moving? false)
              (else
                (Variables|Default|SetCurrentActions (Variables|Default|GetReleasedActions))
                (goto _label))))))
      (else
        (Timeline|PressurePlate%20Timeline Reverse)))
    (else
      (Transformation|SetRelativeLocation (Variables|Default|GetPlate%20Mesh) (Math|Vector|MakeVector 0.0 0.0 (Variables|Default|GetRelative%20Location%20Z)) false false))))

(event Custom|Event%20Reset%20Toggle_FloorGate
  ;[1 1 1] FloorGateのDoOnceをリセット
  (for _array_element (Variables|Default|GetFloorGates)
    (Utilities|IsValid _array_element
      (:Is%20Valid
        (Default|EventResetToggleOpenDoOnce _array_element)))))

(event Custom|Event%20Begin%20Overlap
  (params (Hit%20Actor :type Actor%20Object%20Reference))
  (if (Variables|Default|GetCheckPressed)
    (CallFunction|SetPlayerTriggered Hit%20Actor)
    (CallFunction|SetObjectTriggered Hit%20Actor)
    (CallFunction|EventHit)
    (Utilities|FlowControl|DoOnce false
      (:Completed
        (CallFunction|EventResetToggleShutter)
        (CallFunction|EventResetToggleFloorGate)))))

(event Custom|Event%20End%20Overlap
  (Variables|Default|SetPlayerTriggered false)
  (Variables|Default|SetObjectTriggered false)
  (CallFunction|EventHit)
  (Utilities|FlowControl|DoOnce false) ; enters at Reset
)

(event Custom|Set%20PlayerTriggered
  (params (Hit%20Actor :type Actor%20Object%20Reference))
  (bind _detectplayer (Variables|Default|GetDetectPlayer))
  (Utilities|Casting|CastTo Hit%20Actor)
  (if _detectplayer
    (Variables|Default|SetPlayerTriggered _detectplayer)))

(event Custom|Set%20ObjectTriggered
  (params (Hit%20Actor :type Actor%20Object%20Reference))
  (bind _detectobject (Variables|Default|GetDetectObject))
  (Utilities|Casting|CastTo00_MobiusObject_BP Hit%20Actor)
  (if _detectobject
    (Variables|Default|SetObjectTriggered _detectobject)))

(event Custom|Event%20Reset%20Toggle_Shutter
  (Utilities|FlowControl|DoOnce true) ; enters at Reset
)

(event Custom|Event%20Play%20Sound
  (bind _returnvalue (Transformation|GetActorLocation))
  (if (Variables|Default|GetIs%20Pressed?)
    (Utilities|FlowControl|DoOnce false :!label _label
      (:Completed
        (Utilities|FlowControl|Delay 0.2)
        (Audio|PlaySoundatLocation (Variables|Default|GetPressed%20Sound) _returnvalue "0, 0, 0" 1.0 1.0 0.0 "/Game/17_Kawasaki/Sound/SA_SoundEffect.SA_SoundEffect" 0 0)
        (goto _label_2 Reset)))
    (else
      (Utilities|FlowControl|DoOnce true :!label _label_2
        (:Completed
          (Audio|PlaySoundatLocation (Variables|Default|GetReleased%20Sound) _returnvalue "0, 0, 0" 1.0 1.0 0.0 "/Game/17_Kawasaki/Sound/SA_SoundEffect.SA_SoundEffect" 0 0)
          (goto _label Reset))))))

(event EventBeginPlay
  (if (Variables|Default|GetEnable)
    (|CallParentFunction)))

(event EventTick
  (params (DeltaSeconds :type Float%20%28single-precision%29))
  (bind _asmobius_game_instance (Utilities|Casting|CastToMobiusGameInstance (Game|GetGameInstance)))
  (if (== (Variables|/Game/99_MyContents/BP/MobiusGameInstance.MobiusGameInstance_C|GetCurrentStageNumber _asmobius_game_instance) (Variables|Default|GetStageNumber))
    (if (Variables|Default|GetEnable)
      (CallFunction|PressandRelease)
      (CallFunction|CheckHit)
      (CallFunction|SyncwithParent)
      (CallFunction|EventPlaySound))))

(fn ConstructionScript)

(fn CheckHit
  (bind _returnvalue (Transformation|GetActorLocation))
  (bind (_outhit _returnvalue_2) (Class|KismetSystemLibrary|BoxTraceSingleforObjects _returnvalue (+ _returnvalue (* (Transformation|GetActorUpVector) "0, 0,25.000000")) "40.000000,40.000000,0.000000" "0, 0, 0" (Utilities|Array|MakeArray "ObjectTypeQuery2" "ObjectTypeQuery3") false 0 "None" true))
  (if _returnvalue_2
    (if (Variables|Default|GetCheckPressed)
      (CallFunction|EventBeginOverlap (.HitActor (Collision|BreakHitResult _outhit))))
    (elif (Variables|Default|GetCheckReleased)
      (CallFunction|EventEndOverlap))))

(fn SyncwithParent
  (bind _aspressure_plate_bp (Utilities|Casting|CastToPressurePlate_BP (Actor|GetAttachParentActor)))
  (Variables|Default|SetRelative%20Location%20Z (Variables|PressurePlate_BP_C|GetRelative%20Location%20Z _aspressure_plate_bp)))