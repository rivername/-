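; Key box whose twin doors open on an externally set flag, letting the player collect the key that clears the stage.
; Tick drives paired DoOnce gates with delays that switch the red/green light and play or reverse the door timeline.
; Once the doors finish opening, a per-tick box trace for pawns sets StageCleared on the player character, once.
; An attached box copies its open state from a parent KeyBox_BP; key T is a debug toggle.
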(event Custom|Event%20Door%20Close
  (if (Variables|Default|GetEnableSwitch)
    (Utilities|FlowControl|DoOnce false
      (:Completed
        (Variables|Default|SetEnableSwitch false)
        (Variables|Default|SetIs%20Opening? false)
        (Utilities|FlowControl|Delay 1.5)
        (CallFunction|SetLightState-Close)
        (Variables|Default|SetEnableSwitch true)
        (Utilities|FlowControl|DoOnce false) ; enters at Reset
      ))))

(event Custom|Event%20Door%20Open
  (if (Variables|Default|GetEnableSwitch)
    (Utilities|FlowControl|DoOnce false
      (:Completed
        (Variables|Default|SetEnableSwitch false)
        (CallFunction|SetLightState-Open)
        (Utilities|FlowControl|Delay 1.0)
        (Variables|Default|SetIs%20Opening? true)
        (Utilities|FlowControl|Delay 0.5)
        (Variables|Default|SetEnableSwitch true)
        (Utilities|FlowControl|DoOnce false) ; enters at Reset
      ))))

(event Custom|Event%20Open%20And%20Close
  ;[1 1 1] 開け閉め
  (if (Variables|Default|GetSetOpen)
    (CallFunction|EventDoorOpen)
    (else
      (CallFunction|EventDoorClose)
      (Variables|Default|SetPlayerCanPickUpKey false)))
  (if (Variables|Default|GetIs%20Opening?)
    (bind _rotation_z (Timeline|DoorRotation Play)
      (:Update
        (Transformation|SetWorldRotation (Variables|Default|GetPivot_LeftDoor) (Math|Rotator|MakeRotator 0.0 0.0 _rotation_z) false false)
        (Transformation|SetWorldRotation (Variables|Default|GetPivot_RightDoor) (Math|Rotator|MakeRotator 0.0 0.0 (* _rotation_z -1.0)) false false))
      (:Finished
        (if (> _rotation_z 0.0)
          (Variables|Default|SetPlayerCanPickUpKey true))))
    (else
      (Timeline|DoorRotation Reverse))))

(event Custom|SetOpenState
  (params (SetOpen :type Boolean))
  (Variables|Default|SetSetOpen SetOpen))

(event EventBeginPlay
  (|CallParentFunction))

(event EventTick
  (params (DeltaSeconds :type Float%20%28single-precision%29))
  (CallFunction|EventOpenandClose)
  (CallFunction|CheckPlayerTrigger)
  (CallFunction|SyncwithParent))

(event Input|KeyboardEvents|T
  (params (Key :type Key%20Structure))
  ;[1 1 1] Debug
  (:Pressed
    (CallFunction|SetOpenState true))
  (:Released
    (CallFunction|SetOpenState false)))

(fn ConstructionScript)

(fn SetLightState-Open
  (Rendering|Material|SetMaterial (Variables|Default|GetLight) 0 "/Game/17_Kawasaki/BP/KeyBox/M_GreenLight.M_GreenLight"))

(fn SetLightState-Close
  (Rendering|Material|SetMaterial (Variables|Default|GetLight) 0 "/Game/17_Kawasaki/BP/KeyBox/M_RedLight.M_RedLight"))

(fn CheckPlayerTrigger
  (bind _returnvalue (Transformation|GetActorLocation))
  (bind _returnvalue_2 (Class|KismetSystemLibrary|BoxTraceSingleforObjects _returnvalue (+ _returnvalue (* (Transformation|GetActorForwardVector) "-50.000000,0.000000, 0")) "20.000000,20.000000,20.000000" "0, 0, 0" (Utilities|Array|MakeArray "ObjectTypeQuery3") false 0 "ForOneFrame" true))
  (if _returnvalue_2
    (if (and (Variables|Default|GetPlayerCanPickUpKey) (not (Variables|Default|GetPlayerKeyPickedUp)))
      (bind _asmobius_character (Utilities|Casting|CastTo (Game|GetPlayerCharacter 0)))
      (Variables|Default|SetStageCleared _asmobius_character true)
      (Variables|Default|SetPlayerKeyPickedUp true))))

(fn SyncwithParent
  (bind _askey_box_bp (Utilities|Casting|CastToKeyBox_BP (Actor|GetAttachParentActor)))
  (CallFunction|SetOpenState (Variables|KeyBox_BP_C|GetSetOpen _askey_box_bp)))