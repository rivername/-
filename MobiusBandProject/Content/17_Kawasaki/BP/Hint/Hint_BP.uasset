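; Hint actor that shows per-stage hint text in a UI_Hint widget once the player has spent a set wait time on a stage.
; A looping timer counts seconds, while Tick polls MobiusGameInstance for stage changes, which reset the count, clear the text and re-arm the hint.
; CancelHint suppresses the hint for the matching current stage, and HideHint clears it and restarts the wait.
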(event Custom|Event%20Timer
  (Math|Integer|IncrementInt (Variables|Default|GetElapsed%20Seconds)))

(event Custom|Event%20Hide%20Hint
  (Variables|Default|SetElapsed%20Seconds 0)
  (Default|DestroyText (Variables|Default|GetUI_Hint)))

(event Custom|Event%20Stage%20Changed
  (Variables|Default|SetElapsed%20Seconds 0)
  (Default|DestroyText (Variables|Default|GetUI_Hint))
  (Variables|Default|SetNot%20Need%20to%20Show%20Hint false))

(event Custom|Event%20Show%20Hint
  (bind _ui_hint (Variables|Default|GetUI_Hint))
  (if (>= (Variables|Default|GetElapsed%20Seconds) (Variables|Default|GetSec%20of%20Wait%20for%20Show%20Hint))
    (if (Variables|Default|GetNot%20Need%20to%20Show%20Hint)
      (Default|DestroyText _ui_hint)
      (else
        (Default|SetText _ui_hint (Utilities|Array|Get(acopy) (Variables|Default|GetHint%20Texts) (Variables|Default|GetCurrent%20Stage%20Number%20Prev)))))))

(event Custom|Event%20Cancel%20Hint
  (params (Stage%20Number :type Integer))
  (if (== Stage%20Number (Variables|Default|GetCurrent%20Stage%20Number%20Prev))
    (Variables|Default|SetNot%20Need%20to%20Show%20Hint true)))

(event EventBeginPlay
  (bind _returnvalue (UserInterface|CreateWidget "/Game/17_Kawasaki/BP/Hint/UI_Hint.UI_Hint_C" (Game|GetPlayerController 0)))
  (Default|DestroyText _returnvalue)
  (UserInterface|Viewport|AddtoViewport _returnvalue 0)
  (Variables|Default|SetUI_Hint _returnvalue)
  (Utilities|Time|SetTimerbyEvent (delegate Custom|Event%20Timer) 1.0 true))

(event EventTick
  (params (DeltaSeconds :type Float%20%28single-precision%29))
  (Input|EnableInput (Game|GetPlayerController 0))
  (bind _asmobius_game_instance (Utilities|Casting|CastToMobiusGameInstance (Game|GetGameInstance)))
  (if (!= (Variables|Default|GetCurrent%20Stage%20Number%20Prev) (Variables|/Game/99_MyContents/BP/MobiusGameInstance.MobiusGameInstance_C|GetCurrentStageNumber _asmobius_game_instance))
    (Variables|Default|SetCurrent%20Stage%20Number%20Prev (Variables|/Game/99_MyContents/BP/MobiusGameInstance.MobiusGameInstance_C|GetCurrentStageNumber _asmobius_game_instance))
    (CallFunction|EventStageChanged)
    (else
      (CallFunction|EventShowHint))))

(fn ConstructionScript)