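; A movable object variant that changes its X position as the player moves between rooms.
; On the player character's room-change event, it eases to the offset mapped to that room number, or snaps to a default offset if none exists.
; Reaching the end room key turns on gravity and stops further changes.
; Reset Location shifts it along Y by the player's room number and adds room-offset keys to the map.
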(event Custom|Bind%20Event%20to%20Event%20Player%20Room%20Changed
  (bind _asmobius_character (Utilities|Casting|CastTo (Game|GetPlayerCharacter 0)))
  (EventDispatchers|BindEventtoEventPlayerRoomChanged _asmobius_character (delegate Custom|Event%20Player%20Room%20Changed)))

(event Custom|Event%20Player%20Room%20Changed
  (params (New%20Player%20Room%20Number :type Integer))
  (bind _returnvalue (Transformation|GetActorLocation))
  (bind _returnvalue_2 (Transformation|GetActorLocation))
  (bind _location_x (Variables|Default|GetLocation%20X))
  (bind (_value _returnvalue_3) (Utilities|Map|Find _location_x New%20Player%20Room%20Number))
  (if (not (Variables|Default|GetDone%20Changing))
    (if _returnvalue_3
      (bind _alpha (Timeline|Timeline%20-%20Location%20X PlayFromStart)
        (:Update
          (CallFunction|SetLocationForce (Math|Vector|MakeVector (Math|Float|Lerp (.x _returnvalue_2) (+ _value (Variables|Default|GetInitial%20Location%20X)) _alpha) (.y _returnvalue_2) (.z _returnvalue_2)))
          (if (== New%20Player%20Room%20Number (Variables|Default|GetEnd%20Location%20X%20Key))
            (Variables|Default|SetApply%20Gravity? true)
            (Variables|Default|SetDone%20Changing true))))
      (else
        (CallFunction|SetLocationForce (Math|Vector|MakeVector (+ (Variables|Default|GetInitial%20Location%20X) (Variables|Default|GetDefault%20Relative%20Location%20X)) (.y _returnvalue) (.z _returnvalue)))))))

(event EventBeginPlay
  (|CallParentFunction)
  (CallFunction|BindEventtoEventPlayerRoomChanged))

(event EventTick
  (params (DeltaSeconds :type Float%20%28single-precision%29))
  (|CallParentFunction DeltaSeconds))

(fn ConstructionScript
  (|CallParentFunction)
  (Variables|Default|SetApply%20Gravity? false)
  (Variables|Default|SetInitial%20Location%20X (.x (Transformation|GetActorLocation))))

(fn ResetLocation
  (bind _new_location_x_map (LocalVariables|GetNew%20Location%20X%20Map))
  (bind _asmobius_character (Utilities|Casting|CastTo (Game|GetPlayerCharacter 0)))
  (LocalVariables|SetPlayer%20Room%20Number (Variables|Default|GetPlayerRoomNumber _asmobius_character))
  (Variables|Default|SetApply%20Gravity? false)
  (Variables|Default|SetDone%20Changing false)
  (CallFunction|SetLocationForce (+ (Variables|Default|GetInitialLocation) (Math|Vector|MakeVector 0.0 (* (LocalVariables|GetPlayer%20Room%20Number) 2e+03) 0.0)))
  (bind _keys (Utilities|Map|Keys (Variables|Default|GetLocation%20X)))
  (for (_array_element _array_index) _keys
    (bind _values (Utilities|Map|Values (Variables|Default|GetLocation%20X)))
    (Utilities|Map|Add (LocalVariables|GetNew%20Location%20X%20Map) (+ (LocalVariables|GetPlayer%20Room%20Number) _array_element) (Utilities|Array|Get(acopy) _values _array_index))
    (Variables|Default|SetLocation%20X _new_location_x_map)
    (bind _keys_2 (Utilities|Map|Keys _new_location_x_map))
    (for _array_element_2 _keys_2
      _)))