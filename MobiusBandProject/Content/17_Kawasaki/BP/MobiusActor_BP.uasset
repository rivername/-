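; MobiusActor is a stage actor that repeats itself across neighboring rooms, apparently to give a looping-room illusion.
; On BeginPlay, the IsMain instance spawns attached copies one room width to either side along Y, with the IsMain check preventing endless spawning.
; On RoomChanged, it shifts from its initial location to the player's room number, carrying the copies along, if its stage is current.
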(event Custom|Event%20Room%20Changed
  (CallFunction|MoveActor))

(event EventBeginPlay
  (CallFunction|SpawnActor))

(fn ConstructionScript
  (if (Variables|Default|GetIs%20Main?)
    (Variables|Default|SetInitialLocation (Transformation|GetActorLocation))))

(fn PrintArray
  (params (Array :type Array%20of%20Actor%20Object%20References))
  (for _array_element Array
    (Utilities|Array|Add (LocalVariables|GetStringArray) (Utilities|GetDisplayName _array_element)))
  (Development|PrintString (Utilities|String|JoinStringArray (LocalVariables|GetStringArray) "  / ")))

(fn SpawnActor
  (if (Variables|Default|GetIs%20Main?) ; 無限ループ防止
    (for _index (range -1 1)
      (if (!= _index 0)
        (bind _returnvalue (Game|SpawnActorfromClass (Utilities|GetClass self) (Math|Transform|MakeTransform (+ (Transformation|GetActorLocation) (Math|Vector|MakeVector 0.0 (* _index 2e+03) 0.0)) (Transformation|GetActorRotation) (Transformation|GetActorScale3D)) "AlwaysSpawn" 0 0)) ; 左右にスポーン
        (Transformation|AttachActorToActor _returnvalue self "None" "KeepWorld" "KeepWorld" "KeepWorld" true) ; 親子関係にする
        (Variables|MobiusActor_BP_C|SetStageNumber _returnvalue (Variables|Default|GetStageNumber))))))

(fn MoveActor
  (Variables|Default|SetIs%20Moving? true)
  (if (Variables|Default|GetIs%20Main?)
    ;[1 1 1] 現在のステージのアクタだったら
    (bind _asmobius_game_instance (Utilities|Casting|CastToMobiusGameInstance (Game|GetGameInstance)))
    (if (== (Variables|Default|GetStageNumber) (Variables|/Game/99_MyContents/BP/MobiusGameInstance.MobiusGameInstance_C|GetCurrentStageNumber _asmobius_game_instance))
      (bind _asmobius_character (Utilities|Casting|CastTo (Game|GetPlayerCharacter 0)))
      ;[1 1 1] そのまま変更
      (Transformation|SetActorLocation (+ (Variables|Default|GetInitialLocation) (Math|Vector|MakeVector 0.0 (* (Variables|Default|GetPlayerRoomNumber _asmobius_character) 2e+03) 0.0)) false false))))