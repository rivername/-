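; Base custom-gravity object that falls toward floor or ceiling, following the player's gravity direction.
; While enabled, Tick integrates its own acceleration, flipping G when the player's gravity switches, and pauses during game resets or while the object is moving.
; A line trace from center to bounds edge detects landings, ignoring character meshes, and snaps the object onto the surface.
; A latch plays one landing sound, except on Mobius objects.
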(event EventBeginPlay
  (Variables|Default|SetCurrentLocation (Transformation|GetActorLocation)) ; 現在の座標を保持
  (bind _ascustom_gravity_player_bp (Utilities|Casting|CastToCustomGravityPlayer_BP (Game|GetPlayerCharacter 0)))
  (Variables|Default|SetIs%20Gravity%20True%20Direction? (Variables|/Game/18_Kawana/BP/CustomGravityPlayer_BP.CustomGravityPlayer_BP_C|GetGravity _ascustom_gravity_player_bp)) ; 重力の方向を保持
)

(event EventTick
  (params (DeltaSeconds :type Float%20%28single-precision%29))
  (if (Variables|Default|GetApply%20Gravity?)
    (CallFunction|ApplyGravity)
    (if (Variables|Default|GetIs%20In%20Air?)
      (Variables|Default|SetDO-ONCE true))))

(fn ConstructionScript)

(fn ApplyGravity
  (bind _returnvalue (Transformation|GetActorLocation))
  (bind _returnvalue_2 (Transformation|GetActorLocation))
  (bind _asmobius_game_instance (Utilities|Casting|CastToMobiusGameInstance (Game|GetGameInstance)))
  (if (not (Variables|/Game/99_MyContents/BP/MobiusGameInstance.MobiusGameInstance_C|GetIs%20Reseting? _asmobius_game_instance))
    (if (not (Variables|Default|GetIs%20Moving?)) ; 前後左右に動いていないとき
      ;[1 1 1] 重力の状態
      (bind _ascustom_gravity_player_bp (Utilities|Casting|CastToCustomGravityPlayer_BP (Game|GetPlayerCharacter 0)))
      (if (Math|Boolean|Equal(Boolean) (Variables|Default|GetIs%20Gravity%20True%20Direction?) (Variables|/Game/18_Kawana/BP/CustomGravityPlayer_BP.CustomGravityPlayer_BP_C|GetGravity _ascustom_gravity_player_bp)) ; 重力の切り替えがあったか
        _
        (else
          (Variables|Default|SetG (* -1.0 (Variables|Default|GetG)))
          (Variables|Default|SetIs%20Gravity%20True%20Direction? (Variables|/Game/18_Kawana/BP/CustomGravityPlayer_BP.CustomGravityPlayer_BP_C|GetGravity _ascustom_gravity_player_bp)) ; 現在の重力の方向を保持
        ))
      (Variables|Default|SetAccelaration (- (Variables|Default|GetAccelaration) (* (Variables|Default|GetG) (Utilities|Time|GetWorldDeltaSeconds)))) ; 加速度計算
      (if (>= 0.0 (Variables|Default|GetAccelaration)) ; 上下どっちに落下中？
        ;[1 1 1] 床との当たり判定
        (bind (_outhit _returnvalue_3) (Collision|LineTraceForObjects _returnvalue_2 (- _returnvalue_2 (Math|Vector|MakeVector 0.0 0.0 (.z (.BoxExtent (Collision|GetActorBounds false false))))) (Variables|Default|GetCollisionObjectTypes) false 0 "ForOneFrame"))
        (if _returnvalue_3
          (CallFunction|PlaySoundTrace _outhit)
          ;[1 1 1] MobiusCharacterのmeshとの判定を無視
          (bind _asmobius_character (Utilities|Casting|CastTo (.HitActor (Collision|BreakHitResult _outhit)))
            (:then
              (if (!= (Variables|/Script/Engine.Character|GetMesh _asmobius_character) (.HitComponent (Collision|BreakHitResult _outhit)))
                ;[1 1 1] 着地
                (bind _landlocation (CallFunction|Land (.Location (Collision|BreakHitResult _outhit)) true :!label _label))
                (Transformation|SetActorLocation _landlocation false false)
                (Variables|Default|SetAccelaration 0.0 :!label _label_2)
                (Variables|Default|SetIs%20In%20Air? false)))
            (:CastFailed
              (goto _label)))
          (else
            ;[1 1 1] 落下
            (Transformation|AddActorLocalOffset (Math|Vector|MakeVector 0.0 0.0 (Variables|Default|GetAccelaration)) false false :!label _label_3)
            (Variables|Default|SetIs%20In%20Air? true)))
        (else
          ;[1 1 1] 天井との当たり判定
          (bind (_outhit_2 _returnvalue_4) (Collision|LineTraceForObjects _returnvalue (+ _returnvalue (Math|Vector|MakeVector 0.0 0.0 (.z (.BoxExtent (Collision|GetActorBounds false false))))) (Variables|Default|GetCollisionObjectTypes) false 0 "ForOneFrame"))
          (if _returnvalue_4
            (CallFunction|PlaySoundTrace _outhit_2)
            (bind _asmobius_character_2 (Utilities|Casting|CastTo (.HitActor (Collision|BreakHitResult _outhit_2)))
              (:then
                (if (!= (Variables|/Script/Engine.Character|GetMesh _asmobius_character_2) (.HitComponent (Collision|BreakHitResult _outhit_2)))
                  (bind _landlocation_2 (CallFunction|Land (.Location (Collision|BreakHitResult _outhit_2)) false :!label _label_4))
                  (Transformation|SetActorLocation _landlocation_2 false false)
                  (goto _label_2)))
              (:CastFailed
                (goto _label_4)))
            (else
              (goto _label_3))))))))

(fn Land
  (params (HitLocation :type Vector) (FallDown? :type Boolean))
  (if FallDown? ; 落下の方向で分岐
    ;[1 1 1] 床に着地
    (LocalVariables|SetReturnLocation (+ HitLocation (Math|Vector|MakeVector 0.0 0.0 (.z (.BoxExtent (Collision|GetActorBounds false false))))))
    (else
      ;[1 1 1] 天井に着地
      (LocalVariables|SetReturnLocation (- HitLocation (Math|Vector|MakeVector 0.0 0.0 (.z (.BoxExtent (Collision|GetActorBounds false false))))))))
  (return (LocalVariables|GetReturnLocation)))

(fn PlaySoundTrace
  (params (Hit%20Result :type Hit%20Result%20Structure))
  (Utilities|Casting|CastTo00_MobiusObject_BP (.HitActor (Collision|BreakHitResult Hit%20Result))
    (:CastFailed
      (if (Variables|Default|GetDO-ONCE)
        (Variables|Default|SetDO-ONCE false)
        (CallFunction|PlaySound "NewEnumerator1")))))