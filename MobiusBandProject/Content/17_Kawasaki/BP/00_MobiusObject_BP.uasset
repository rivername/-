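; Grabbable puzzle block for the Mobius rooms that the player pushes or pulls along the X/Y axes.
; Each tick, box and line traces find the player's side and facing to drive the outline, player snapping and axis input.
; Timeline moves carry block and player after obstacle or ledge checks, then round to a grid.
; It also follows Mobius objects stacked along gravity and jumps to its left or right side mesh when that overlaps a matching actor.
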(event Custom|Event%20Start%20Snap%20Player
  (params (Player%20Location :type Vector) (New%20Location :type Vector) (New%20Rotation :type Rotator))
  ;[1 1 1] 時間をかけてスナップする
  (Variables|Default|SetDone%20Snapping false)
  (bind _alpha (Timeline|Snap%20Player%20Timeline PlayFromStart)
    (:Update
      (Transformation|SetActorLocationAndRotation (Game|GetPlayerCharacter 0) (Math|Vector|Lerp(Vector) Player%20Location New%20Location _alpha) New%20Rotation))
    (:Finished
      (Variables|Default|SetDone%20Snapping true))))

(event Custom|MoveObjectAndPlayer
  (params (Push? :type Boolean) (Pull? :type Boolean) (Right :type Boolean) (Left :type Boolean) (Fore :type Boolean) (Back :type Boolean))
  (bind _returnvalue (Transformation|GetActorLocation))
  (bind _returnvalue_2 (Game|GetPlayerCharacter 0))
  (bind _returnvalue_3 (Transformation|GetActorLocation))
  (bind _tracedirection (Variables|Default|GetTraceDirection))
  (bind _tracedirection_2 (Variables|Default|GetTraceDirection))
  (bind _returnvalue_4 (Transformation|GetActorLocation _returnvalue_2))
  (bind _returnvalue_5 (* _tracedirection_2 -1.0))
  (bind _returnvalue_6 (Transformation|GetActorUpVector _returnvalue_2))
  (bind _charactermovement (Variables|/Script/Engine.Character|GetCharacterMovement _returnvalue_2))
  (bind _returnvalue_7 (* _returnvalue_6 (Math|Vector|MakeVector 0.0 0.0 (.z _returnvalue_5))))
  (bind _returnvalue_8 (+ _returnvalue_4 _returnvalue_7))
  (if (Variables|Default|GetIs%20In%20Air?) ; 空中にいると移動できない
    (CallFunction|SetGrabingStateNone)
    (else
      ;[1 1 1] 押したり引いたりしてなかったら
      (bind _asmobius_character (Utilities|Casting|CastTo _returnvalue_2))
      (if (not (or (Variables|Default|GetIs%20Pushing? _asmobius_character) (Variables|Default|GetIs%20Pulling? _asmobius_character)))
        ;[1 1 1] プレイヤーの状態をセットする
        (Variables|Default|SetIs%20Pushing? _asmobius_character Push?)
        (Variables|Default|SetIs%20Pulling? _asmobius_character Pull?)
        (if Push?
          ;[1 1 1] 押す
          (Variables|Default|SetPlayerMoveScaleValue 1.0)
          (else
            ;[1 1 1] 引く
            (Variables|Default|SetPlayerMoveScaleValue 0.1)))
        (if Right
          ;[1 1 1] 動かす方向をセット
          (Variables|Default|SetWorldDirection "0,1.000000,1.000000")
          (if (not (Variables|Default|GetDO_ONCE)) :!label _label
            (Variables|Default|SetDO_ONCE true)
            (if Push?
              ;[1 1 1] 押す ： 動かせるかチェック（オブジェクト基準）
              (bind (_outhit _returnvalue_9) (Collision|LineTraceForObjects (+ _returnvalue (Math|Vector|MakeVector 0.0 0.0 (.Z (Math|Vector|BreakVector _tracedirection)))) (+ _returnvalue (* _tracedirection (Variables|Default|GetWorldDirection))) (Utilities|Array|MakeArray "ObjectTypeQuery2") false 0 "None"))
              (if _returnvalue_9
                ;[1 1 1] MoveForceの場合壁だけ判定
                (if (Variables|Default|GetMove%20Force)
                  (Utilities|Casting|CastToMobiusRoom (.HitActor (Collision|BreakHitResult _outhit))
                    (:then
                      ;[1 1 1] 動かせなかったら
                      (bind _asmobius_character_2 (Utilities|Casting|CastTo _returnvalue_2 :!label _label_2))
                      (Variables|Default|SetIs%20Pushing? _asmobius_character_2 false)
                      (Variables|Default|SetIs%20Pulling? _asmobius_character_2 false)
                      (CallFunction|SetGrabingStateNone)
                      (Variables|Default|SetDO_ONCE false))
                    (:CastFailed
                      ;[1 1 1] 移動先を取得
                      (bind _output_get (Variables|Default|SetTargetLocation_Prev _returnvalue :!label _label_3))
                      (bind _value (Timeline|PushTimeline PlayFromStart)
                        (:Update
                          (bind _output_get_2 (Variables|Default|SetTargetLocation (+ _output_get (* (Math|Vector|MakeVector _value _value 0.0) (Variables|Default|GetWorldDirection)))))
                          ;[1 1 1] プレイヤーを移動
                          (Transformation|SetActorLocation _returnvalue_2 (Math|Vector|MakeVector (.X (Math|Vector|BreakVector (+ (* (Math|Vector|MakeVector (Math|Conversions|ToFloat(Integer) (Math|Float|Round (.x (Math|Vector|GetUnitDirection(Vector) (Variables|Default|GetTargetLocation) (Transformation|GetActorLocation (Game|GetPlayerCharacter 0)))))) (Math|Conversions|ToFloat(Integer) (Math|Float|Round (.y (Math|Vector|GetUnitDirection(Vector) (Variables|Default|GetTargetLocation) (Transformation|GetActorLocation (Game|GetPlayerCharacter 0)))))) 0.0) "100.000000,100.000000, 0") _output_get_2))) (.Y (Math|Vector|BreakVector (+ (* (Math|Vector|MakeVector (Math|Conversions|ToFloat(Integer) (Math|Float|Round (.x (Math|Vector|GetUnitDirection(Vector) (Variables|Default|GetTargetLocation) (Transformation|GetActorLocation (Game|GetPlayerCharacter 0)))))) (Math|Conversions|ToFloat(Integer) (Math|Float|Round (.y (Math|Vector|GetUnitDirection(Vector) (Variables|Default|GetTargetLocation) (Transformation|GetActorLocation (Game|GetPlayerCharacter 0)))))) 0.0) "100.000000,100.000000, 0") _output_get_2))) (.z (Transformation|GetActorLocation _returnvalue_2))) false false)
                          ;[1 1 1] プレイヤーの向きを移動方向にする -> 無効
                          (Variables|/Script/Engine.CharacterMovementComponent|SetbOrientRotationToMovement _charactermovement false)
                          (Variables|Default|SetIs%20Moving? true) ; 移動中にする
                          ;[1 1 1] 移動音を再生
                          (Utilities|FlowControl|DoOnce false :!label _label_4
                            (:Completed
                              (CallFunction|PlaySound "NewEnumerator0"))))
                        (:Finished
                          (Variables|Default|SetDO_ONCE false)
                          (Variables|Default|SetTargetLocation_Prev _returnvalue)
                          ;[1 1 1] プレイヤーの向きを移動方向にする -> 有効
                          (Variables|/Script/Engine.CharacterMovementComponent|SetbOrientRotationToMovement _charactermovement true)
                          ;[1 1 1] 状態をリセット
                          (bind _asmobius_character_3 (Utilities|Casting|CastTo _returnvalue_2))
                          (Variables|Default|SetIs%20Pushing? _asmobius_character_3 false)
                          (Variables|Default|SetIs%20Pulling? _asmobius_character_3 false)
                          (Variables|Default|SetIs%20Moving? false) ; 移動中を解除
                          (bind _fit (CallFunction|FitLocation (Math|Vector|MakeVector (.x _returnvalue_3) (.y _returnvalue_3) 0.0)))
                          (CallFunction|SetLocationForce (Math|Vector|MakeVector (.x _fit) (.y _fit) (.z _returnvalue_3)))
                          (if (Variables|Default|GetIs%20PlayerGrabing?)
                            (goto _label_4 Reset)
                            (else
                              (CallFunction|SetGrabingStateNone)
                              (goto _label_4 Reset)))))))
                  (else
                    (goto _label_2)))
                (else
                  ;[1 1 1] 重力が無効の時穴に落ちないようにする
                  (if (Variables|Default|GetApply%20Gravity?)
                    (goto _label_3)
                    (else
                      (bind _returnvalue_10 (Collision|LineTraceForObjects (+ (Transformation|GetActorLocation) (* (Variables|Default|GetWorldDirection) "100.000000,100.000000,0.000000")) (+ (+ (Transformation|GetActorLocation) (* (Variables|Default|GetWorldDirection) "100.000000,100.000000,0.000000")) (* (Transformation|GetActorUpVector) "0, 0,-100.000000")) (Utilities|Array|MakeArray "ObjectTypeQuery1" "ObjectTypeQuery2") false 0 "None"))
                      (if _returnvalue_10
                        (goto _label_3)
                        (else
                          (goto _label_2)))))))
              (else
                ;[1 1 1] 引く ： 動かせるかチェック（プレイヤー基準）
                (bind _returnvalue_11 (Collision|LineTraceForObjects _returnvalue_8 (+ _returnvalue_8 (* (Transformation|GetActorForwardVector _returnvalue_2) (.x _returnvalue_5))) (Utilities|Array|MakeArray "ObjectTypeQuery2") false 0 "None"))
                (if _returnvalue_11
                  (goto _label_2)
                  (else
                    (goto _label_3))))))
          (elif Left
            (Variables|Default|SetWorldDirection "0.000000,-1.000000,1.000000")
            (goto _label)
            (elif Fore
              (Variables|Default|SetWorldDirection "-1.000000,0.000000,1.000000")
              (goto _label)
              (elif Back
                (Variables|Default|SetWorldDirection "1.000000,0.000000,1.000000")
                (goto _label)))))))))

(event Custom|SetGrabingStateNone
  ;[1 1 1] つかみ状態をリセット
  (if (Variables|Default|GetIs%20PlayerFacing?)
    (bind _asmobius_character (Utilities|Casting|CastTo (Game|GetPlayerCharacter 0)))
    (if (not (or (Variables|Default|GetIs%20Pushing? _asmobius_character) (Variables|Default|GetIs%20Pulling? _asmobius_character)))
      (Variables|Default|SetIs%20Grabed? _asmobius_character false))))

(event Custom|Event%20Player%20Room%20Changed
  (params (New%20Player%20Room%20Number :type Integer))
  (CallFunction|SetActiveFlag))

(event EventTick
  (params (DeltaSeconds :type Float%20%28single-precision%29))
  (bind _targetlocation (Variables|Default|GetTargetLocation))
  ;[1 1 1] Event Tick
  (|CallParentFunction DeltaSeconds) ; 親クラスのEventTickを実行
  (CallFunction|CheckSideMeshHit)
  (CallFunction|CheckPlayerHit)
  (CallFunction|GetPlayerFacing)
  (CallFunction|GetPushing-Pulling)
  (Transformation|SetActorLocation (Math|Vector|MakeVector (.x _targetlocation) (.y _targetlocation) (.z (Transformation|GetActorLocation))) false false)
  (CallFunction|SetOutline)
  (CallFunction|MoveTogether))

(event EventBeginPlay
  (|CallParentFunction)
  (CallFunction|SetRandomRotation)
  (bind _asmobius_character (Utilities|Casting|CastTo (Game|GetPlayerCharacter 0)))
  (EventDispatchers|BindEventtoEventPlayerRoomChanged _asmobius_character (delegate Custom|Event%20Player%20Room%20Changed)))

(event Input|ActionEvents|InputActionGrabObject
  (params (Key :type Key%20Structure))
  ;[1 1 1] Grabキー入力
  (:Pressed
    (bind _asmobius_character (Utilities|Casting|CastTo (Game|GetPlayerCharacter 0)))
    (if (not (Variables|/Game/18_Kawana/BP/CustomGravityPlayer_BP.CustomGravityPlayer_BP_C|GetJumping _asmobius_character)) ; ジャンプ中じゃなかったら
      (Variables|Default|SetIs%20PlayerGrabing? true)
      (if (Variables|Default|GetIs%20PlayerFacing?)
        (CallFunction|SnapPlayer)
        (bind _returnvalue (Actor|GetActorOfClass "/Game/17_Kawasaki/BP/Hint/Hint_BP.Hint_BP_C"))
        (Default|EventCancelHint _returnvalue))))
  (:Released
    (Variables|Default|SetIs%20PlayerGrabing? false)
    ;[1 1 1] つかみ状態をリセット
    (bind _asmobius_character_2 (Utilities|Casting|CastTo (Game|GetPlayerCharacter 0)))
    (if (not (or (Variables|Default|GetIs%20Pushing? _asmobius_character_2) (Variables|Default|GetIs%20Pulling? _asmobius_character_2)))
      (Variables|Default|SetIs%20Grabed? _asmobius_character_2 false))))

(fn ConstructionScript
  (bind _returnvalue (Transformation|GetActorLocation))
  (Variables|Default|SetTargetLocation _returnvalue)
  (Variables|Default|SetInitialLocation _returnvalue))

(fn SetRandomRotation
  (if (Variables|Default|GetRandom%20Rotation)
    _))

(fn CheckPlayerHit
  (bind _returnvalue (Transformation|GetActorLocation))
  (bind (_array_element _array_index) (Utilities|Array|ForEachLoopwithBreak (Utilities|Array|MakeArray (Math|Vector|MakeVector 1.0 0.0 0.0) (Math|Vector|MakeVector -1.0 0.0 0.0) (Math|Vector|MakeVector 0.0 1.0 0.0) (Math|Vector|MakeVector 0.0 -1.0 0.0)) :!label _label)
    (:LoopBody
      (bind _returnvalue_2 (Class|KismetSystemLibrary|BoxTraceSingleforObjects _returnvalue (+ _returnvalue (* _array_element "80.000000,80.000000,0.000000")) "20.000000,20.000000,20.000000" "0, 0, 0" (Utilities|Array|MakeArray "ObjectTypeQuery3") false 0 "None" true))
      (if _returnvalue_2
        (Variables|Default|SetBackSideTriggered (Utilities|Select :Index _array_index :Option%200 (Variables|Default|GetDetectBack) :Option%201 false :Option%202 false :Option%203 false))
        (Variables|Default|SetForeSideTriggered (Utilities|Select :Index _array_index :Option%200 false :Option%201 (Variables|Default|GetDetectFore) :Option%202 false :Option%203 false))
        (Variables|Default|SetRightSideTriggered (Utilities|Select :Index _array_index :Option%200 false :Option%201 false :Option%202 (Variables|Default|GetDetectRight) :Option%203 false))
        (Variables|Default|SetLeftSideTriggered (Utilities|Select :Index _array_index :Option%200 false :Option%201 false :Option%202 false :Option%203 (Variables|Default|GetDetectLeft)))
        (LocalVariables|SetPlayerHit true)
        (goto _label Break)))
    (:Completed
      (if (not (LocalVariables|GetPlayerHit))
        (Variables|Default|SetBackSideTriggered false)
        (Variables|Default|SetForeSideTriggered false)
        (Variables|Default|SetRightSideTriggered false)
        (Variables|Default|SetLeftSideTriggered false)
        (CallFunction|SetGrabingStateNone)))))

(fn GetPlayerFacing
  (bind _returnvalue (Game|GetPlayerCharacter 0))
  (bind _returnvalue_2 (Transformation|GetActorLocation _returnvalue))
  (bind _returnvalue_3 (Transformation|GetActorUpVector _returnvalue))
  (bind _returnvalue_4 (* "0.000000,0.000000,-50.000000" _returnvalue_3))
  (bind _returnvalue_5 (+ _returnvalue_2 _returnvalue_4))
  ;[1 1 1] プレイヤーの前方のVectorを取得
  (Utilities|IsValid _returnvalue
    (:Is%20Valid
      ;[1 1 1] 自分の方を向いていたら
      (bind (_outhit _returnvalue_6) (Collision|LineTraceForObjects _returnvalue_5 (+ _returnvalue_5 (* (Transformation|GetActorForwardVector _returnvalue) 1e+02)) (Utilities|Array|MakeArray "ObjectTypeQuery2") false 0 "None" false))
      (if (== (.HitActor (Collision|BreakHitResult _outhit)) self)
        (Variables|Default|SetIs%20PlayerFacing? _returnvalue_6)
        ;[1 1 1] PlayerInputを有効化
        (Input|EnableInput (Game|GetPlayerController 0))
        (else
          (Variables|Default|SetIs%20PlayerFacing? false))))))

(fn SnapPlayer
  (bind _returnvalue (Game|GetPlayerCharacter 0))
  (bind _returnvalue_2 (Transformation|GetActorLocation))
  (bind _returnvalue_3 (Transformation|GetActorLocation _returnvalue))
  (bind _returnvalue_4 (+ _returnvalue_2 "0,100.000000, 0"))
  (bind _returnvalue_5 (+ _returnvalue_2 "0,-100.000000,0.000000"))
  (bind _returnvalue_6 (+ _returnvalue_2 "-100.000000,0.000000, 0"))
  (bind _returnvalue_7 (+ _returnvalue_2 "100.000000, 0, 0"))
  (bind _returnvalue_8 (Math|Vector|MakeVector (.x _returnvalue_3) (.y _returnvalue_3) (.z _returnvalue_3)))
  ;[1 1 1] プレイヤーが右にいる
  (if (Variables|Default|GetRightSideTriggered)
    (CallFunction|EventStartSnapPlayer _returnvalue_8 (Math|Vector|MakeVector (.x _returnvalue_4) (.y _returnvalue_4) (.z _returnvalue_3)) "0.000000,270.000000,0.000000")
    (bind _asmobius_character (Utilities|Casting|CastTo _returnvalue))
    (Variables|Default|SetIs%20Grabed? _asmobius_character true)
    (else
      ;[1 1 1] プレイヤーが左にいる
      (if (Variables|Default|GetLeftSideTriggered)
        (CallFunction|EventStartSnapPlayer _returnvalue_8 (Math|Vector|MakeVector (.x _returnvalue_5) (.y _returnvalue_5) (.z _returnvalue_3)) "0.000000,90.000000,0.000000")
        (bind _asmobius_character_2 (Utilities|Casting|CastTo _returnvalue))
        (Variables|Default|SetIs%20Grabed? _asmobius_character_2 true)
        (else
          ;[1 1 1] プレイヤーが手前にいる
          (if (Variables|Default|GetForeSideTriggered)
            (CallFunction|EventStartSnapPlayer _returnvalue_8 (Math|Vector|MakeVector (.x _returnvalue_6) (.y _returnvalue_6) (.z _returnvalue_3)) "0, 0, 0")
            (bind _asmobius_character_3 (Utilities|Casting|CastTo _returnvalue))
            (Variables|Default|SetIs%20Grabed? _asmobius_character_3 true)
            (else
              ;[1 1 1] プレイヤーが奥にいる
              (if (Variables|Default|GetBackSideTriggered)
                (CallFunction|EventStartSnapPlayer _returnvalue_8 (Math|Vector|MakeVector (.x _returnvalue_7) (.y _returnvalue_7) (.z _returnvalue_3)) "0,180.000000, 0")
                (bind _asmobius_character_4 (Utilities|Casting|CastTo _returnvalue))
                (Variables|Default|SetIs%20Grabed? _asmobius_character_4 true)))))))))

(fn GetPushing-Pulling
  (if (Variables|Default|GetIs%20PlayerFacing?)
    (if (Variables|Default|GetDone%20Snapping)
      ;[1 1 1] プレイヤーが右にいる
      (if (Variables|Default|GetRightSideTriggered)
        (bind _asmobius_character (Utilities|Casting|CastTo (Game|GetPlayerCharacter 0)))
        (if (Variables|Default|GetIs%20Grabed? _asmobius_character)
          (if (== (Variables|Default|GetAxisValue_MoveRight _asmobius_character) -1.0)
            ;[1 1 1] Push
            (CallFunction|MoveObjectandPLayer true false false true false false)
            (elif (== (Variables|Default|GetAxisValue_MoveRight _asmobius_character) 1.0)
              ;[1 1 1] Pull
              (CallFunction|MoveObjectandPLayer false true true false false false))))
        (else
          ;[1 1 1] プレイヤーが左にいる
          (if (Variables|Default|GetLeftSideTriggered)
            (bind _asmobius_character_2 (Utilities|Casting|CastTo (Game|GetPlayerCharacter 0)))
            (if (Variables|Default|GetIs%20Grabed? _asmobius_character_2)
              (if (== (Variables|Default|GetAxisValue_MoveRight _asmobius_character_2) 1.0)
                (CallFunction|MoveObjectandPLayer true false true false false false)
                (elif (== (Variables|Default|GetAxisValue_MoveRight _asmobius_character_2) -1.0)
                  (CallFunction|MoveObjectandPLayer false true false true false false))))
            (else
              ;[1 1 1] プレイヤーが手前にいる
              (if (Variables|Default|GetForeSideTriggered)
                (bind _asmobius_character_3 (Utilities|Casting|CastTo (Game|GetPlayerCharacter 0)))
                (if (Variables|Default|GetIs%20Grabed? _asmobius_character_3)
                  (if (== (Variables|Default|GetAxisValue_MoveForward _asmobius_character_3) 1.0)
                    (CallFunction|MoveObjectandPLayer true false false false false true)
                    (elif (== (Variables|Default|GetAxisValue_MoveForward _asmobius_character_3) -1.0)
                      (CallFunction|MoveObjectandPLayer false true false false true false))))
                (else
                  ;[1 1 1] プレイヤーが奥にいる
                  (if (Variables|Default|GetBackSideTriggered)
                    (bind _asmobius_character_4 (Utilities|Casting|CastTo (Game|GetPlayerCharacter 0)))
                    (if (Variables|Default|GetIs%20Grabed? _asmobius_character_4)
                      (if (== (Variables|Default|GetAxisValue_MoveForward _asmobius_character_4) -1.0)
                        (CallFunction|MoveObjectandPLayer true false false false true false)
                        (elif (== (Variables|Default|GetAxisValue_MoveForward _asmobius_character_4) 1.0)
                          (CallFunction|MoveObjectandPLayer false true false false false true))))))))))))))

(fn FitLocation
  (params (Location :type Vector))
  (bind _returnvalue (/ Location 5e+01))
  (return (* (Math|Vector|MakeVector (Math|Conversions|ToFloat(Integer) (Math|Float|Round (.x _returnvalue))) (Math|Conversions|ToFloat(Integer) (Math|Float|Round (.y _returnvalue))) (Math|Conversions|ToFloat(Integer) (Math|Float|Round (.z _returnvalue)))) 5e+01)))

(fn SetLocationForce
  (params (NewLocation :type Vector))
  (Variables|Default|SetTargetLocation NewLocation)
  (bind _output_get (Variables|Default|SetTargetLocation_Prev NewLocation))
  (Transformation|SetActorLocation _output_get false false))

(fn ResetLocation
  (bind _asmobius_character (Utilities|Casting|CastTo (Game|GetPlayerCharacter 0)))
  (CallFunction|SetLocationForce (+ (Variables|Default|GetInitialLocation) (Math|Vector|MakeVector 0.0 (* (Variables|Default|GetPlayerRoomNumber _asmobius_character) 2e+03) 0.0)))
  (Transformation|SetActorLocation (+ (Variables|Default|GetInitialLocation) (Math|Vector|MakeVector 0.0 (* (Variables|Default|GetPlayerRoomNumber _asmobius_character) 2e+03) 0.0)) false false))

(fn MoveTogether
  (bind _returnvalue (Transformation|GetActorLocation))
  (bind _asmobius_character (Utilities|Casting|CastTo (Game|GetPlayerCharacter 0)))
  (if (Variables|/Game/18_Kawana/BP/CustomGravityPlayer_BP.CustomGravityPlayer_BP_C|GetGravity _asmobius_character)
    (LocalVariables|SetL:WorldDirection "0.000000,0.000000,-100.000000")
    (else
      (LocalVariables|SetL:WorldDirection "0.000000,0.000000,100.000000")))
  (bind _outhit (Collision|LineTraceForObjects _returnvalue (+ _returnvalue (LocalVariables|GetL:WorldDirection)) (Utilities|Array|MakeArray "ObjectTypeQuery2") false 0 "None"))
  (bind _as00_mobius_object_bp (Utilities|Casting|CastTo00_MobiusObject_BP (.HitActor (Collision|BreakHitResult _outhit)))
    (:then
      (CallFunction|SetLocationForce (Math|Vector|MakeVector (.x (Transformation|GetActorLocation _as00_mobius_object_bp)) (.y (Transformation|GetActorLocation _as00_mobius_object_bp)) (.z (Transformation|GetActorLocation)))))
    (:CastFailed
      (CallFunction|SetOutline))))

(fn SetOutline
  (bind _staticmesh_center (Variables|Default|GetStaticMesh_Center))
  (if (Variables|Default|GetActive)
    (Utilities|Casting|CastToMobiusGameInstance (Game|GetGameInstance))
    (if (Variables|Default|GetIs%20PlayerFacing?)
      (Rendering|SetRenderCustomDepth _staticmesh_center true)
      (else
        (Rendering|SetRenderCustomDepth _staticmesh_center false)))))

(fn CheckSideMeshHit
  (bind _staticmesh_right (Variables|Default|GetStaticMesh_Right))
  (bind _staticmesh_left (Variables|Default|GetStaticMesh_Left))
  (bind _returnvalue (Transformation|GetWorldLocation _staticmesh_left))
  (bind _returnvalue_2 (Transformation|GetWorldLocation _staticmesh_right))
  ;[1 1 1] 右のMeshとのヒット
  (bind (_outhit _returnvalue_3) (Class|KismetSystemLibrary|BoxTraceSingleforObjects _returnvalue_2 _returnvalue_2 (* (.Max (Components|StaticMesh|GetLocalBounds _staticmesh_right)) 2.0) "0, 0, 0" (LocalVariables|GetCollision%20Object%20Types) false 0 "ForOneFrame" true))
  (if _returnvalue_3
    (Utilities|Casting|CastTo (.HitActor (Collision|BreakHitResult _outhit)))
    (CallFunction|SetLocationForce (Transformation|GetWorldLocation (Variables|Default|GetStaticMesh_Right)))
    (else
      ;[1 1 1] 左のMeshとのヒット
      (bind (_outhit_2 _returnvalue_4) (Class|KismetSystemLibrary|BoxTraceSingleforObjects _returnvalue _returnvalue (* (.Max (Components|StaticMesh|GetLocalBounds _staticmesh_left)) 2.0) "0, 0, 0" (LocalVariables|GetCollision%20Object%20Types) false 0 "ForOneFrame" true))
      (if _returnvalue_4
        (Utilities|Casting|CastTo (.HitActor (Collision|BreakHitResult _outhit_2)))
        (CallFunction|SetLocationForce (Transformation|GetWorldLocation (Variables|Default|GetStaticMesh_Left)))))))

(fn SetActiveFlag
  (bind _asmobius_game_instance (Utilities|Casting|CastToMobiusGameInstance (Game|GetGameInstance)))
  (if (Variables|/Game/99_MyContents/BP/MobiusGameInstance.MobiusGameInstance_C|GetNeedToChangeStage _asmobius_game_instance)
    (if (== (Variables|/Game/99_MyContents/BP/MobiusGameInstance.MobiusGameInstance_C|GetCurrentStageNumber _asmobius_game_instance) (Variables|Default|GetStage%20Number))
      (Variables|Default|SetActive false))))