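; Magic door actor that slides two panels apart or together, with spatialized sounds, and destroys itself once closed.
; SetOpenState drives a timeline forward or in reverse and toggles capture-on-movement on the Capture_BP scene capture.
; Tick calls the binding to the player's room-change event, whose handler requests blocking collision on an open door, then only delays.
; SetDoorCollision's collision calls are disconnected, so it changes nothing.
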(event Custom|Event%20Play%20Sound%20At%20Location
  (params (Sound%20Base :type Sound%20Base%20Object%20Reference))
  (Audio|PlaySoundatLocation Sound%20Base (Transformation|GetActorLocation) "0, 0, 0" 1.0 1.0 0.0 "/Game/17_Kawasaki/Sound/SA_SoundEffect.SA_SoundEffect" 0 0))

(event Custom|Event%20Set%20Open%20State
  (params (Set%20Open :type Boolean))
  ;[1 1 1] Close And Open
  (bind _returnvalue (Actor|GetActorOfClass "/Game/17_Kawasaki/BP/MagicDoor/Capture_BP.Capture_BP_C"))
  (Variables|/Script/Engine.SceneCaptureComponent|SetbCaptureOnMovement (Variables|/Game/17_Kawasaki/BP/MagicDoor/Capture_BP.Capture_BP_C|GetSceneCaptureComponent2D _returnvalue) Set%20Open)
  (if Set%20Open
    (bind _relative_location_x (Timeline|Relative%20Location Play)
      (:Update
        (Transformation|SetRelativeLocation (Variables|Default|GetDoor%20Back) (Math|Vector|MakeVector _relative_location_x 0.0 0.0) false false)
        (Transformation|SetRelativeLocation (Variables|Default|GetDoor%20Fore) (Math|Vector|MakeVector (* _relative_location_x -1.0) 0.0 0.0) false false))
      (:Finished
        (bind _output_get (Variables|Default|SetIs%20Opened? Set%20Open))
        (if _output_get
          (CallFunction|EventPlaySoundatLocation "/Game/17_Kawasaki/Sound/WAV_MagicDoorOpen.WAV_MagicDoorOpen")
          (else
            (Actor|DestroyActor) ; 閉まったらDestroy
            (CallFunction|EventPlaySoundatLocation "/Game/17_Kawasaki/Sound/WAV_MagicDoorClose.WAV_MagicDoorClose")))))
    (else
      (CallFunction|EventPlaySoundatLocation "/Game/17_Kawasaki/Sound/WAV_MagicDoorClose.WAV_MagicDoorClose")
      (Timeline|Relative%20Location Reverse))))

(event Custom|Event%20Player%20Room%20Changed
  (params (New%20Player%20Room%20Number :type Integer))
  ;[1 1 1] Event Player Room Changed
  (if (Variables|Default|GetIs%20Opened?) ; 開いてる場合
    (CallFunction|SetDoorCollision true) ; 通れなくする
    (Utilities|FlowControl|Delay 2.5)))

(event Custom|Bind%20Event%20Player%20Room%20Changed
  ;[1 1 1] Event Player Room Changed
  (bind _asmobius_character (Utilities|Casting|CastTo (Game|GetPlayerCharacter 0)))
  (EventDispatchers|BindEventtoEventPlayerRoomChanged _asmobius_character (delegate Custom|Event%20Player%20Room%20Changed)))

(event EventBeginPlay
  ;[1 1 1] Begin Play
  (CallFunction|SetDoorCollision false))

(event EventTick
  (params (DeltaSeconds :type Float%20%28single-precision%29))
  ;[1 1 1] Event Tick
  (CallFunction|BindEventPlayerRoomChanged))

(fn ConstructionScript)

(fn SetDoorCollision
  (params (Set%20Colision :type Boolean))
  (if Set%20Colision
    _))