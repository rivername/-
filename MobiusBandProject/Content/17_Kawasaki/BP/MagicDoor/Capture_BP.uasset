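; Capture actor for the Magic Door that follows the camera setup from a vertically offset position, presumably to render the door's view.
; Every Tick it copies the CameraController's target rotation with yaw flipped 180 degrees and sets its height from the active top or bottom camera plus a large offset.
; On player room changes needing a stage change, it waits briefly, then moves to the CaptureLocations entry indexed one past the current stage.
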(event Custom|Bind%20Event%20Player%20Room%20Changed
  (bind _asmobius_character (Utilities|Casting|CastTo (Game|GetPlayerCharacter 0)))
  (EventDispatchers|BindEventtoEventPlayerRoomChanged _asmobius_character (delegate Custom|Event%20Player%20Room%20Changed))
  (bind _asmobius_game_instance (Utilities|Casting|CastToMobiusGameInstance (Game|GetGameInstance))))

(event Custom|Event%20Player%20Room%20Changed
  (params (New%20Player%20Room%20Number :type Integer))
  (if (Variables|/Game/99_MyContents/BP/MobiusGameInstance.MobiusGameInstance_C|GetNeedToChangeStage (stale Custom|Bind%20Event%20Player%20Room%20Changed _asmobius_game_instance))
    (Utilities|FlowControl|Delay 0.5)
    (bind _asmobius_game_instance (Utilities|Casting|CastToMobiusGameInstance (Game|GetGameInstance)))
    (Utilities|IsValid (Utilities|Array|Get(acopy) (Variables|Default|GetCapture%20Locations) (+ (Variables|/Game/99_MyContents/BP/MobiusGameInstance.MobiusGameInstance_C|GetCurrentStageNumber _asmobius_game_instance) 1))
      (:Is%20Valid
        (Transformation|SetActorLocation (Transformation|GetActorLocation (Utilities|Array|Get(acopy) (Variables|Default|GetCapture%20Locations) (+ (Variables|/Game/99_MyContents/BP/MobiusGameInstance.MobiusGameInstance_C|GetCurrentStageNumber _asmobius_game_instance) 1))) false false)))))

(event EventBeginPlay
  (Input|EnableInput (Game|GetPlayerController 0))
  (CallFunction|BindEventPlayerRoomChanged))

(event EventTick
  (params (DeltaSeconds :type Float%20%28single-precision%29))
  (CallFunction|SetLocationandRotation))

(fn ConstructionScript)

(fn SetLocationandRotation
  (bind _returnvalue (Transformation|GetActorLocation))
  (bind _returnvalue_2 (Transformation|GetActorLocation))
  (bind _returnvalue_3 (Actor|GetActorOfClass "/Game/99_MyContents/CAMERA/CameraController.CameraController_C"))
  (Variables|Default|SetTarget%20Rotation (Math|Rotator|MakeRotator (.Roll (Math|Rotator|BreakRotator (Variables|/Game/99_MyContents/CAMERA/CameraController.CameraController_C|GetCameraRotationTarget _returnvalue_3))) (.Pitch (Math|Rotator|BreakRotator (Variables|/Game/99_MyContents/CAMERA/CameraController.CameraController_C|GetCameraRotationTarget _returnvalue_3))) (+ (.Yaw (Math|Rotator|BreakRotator (Variables|/Game/99_MyContents/CAMERA/CameraController.CameraController_C|GetCameraRotationTarget _returnvalue_3))) 1.8e+02)))
  (if (Utilities|Enum|Equal(Enum) (Variables|/Game/99_MyContents/CAMERA/CameraController.CameraController_C|GetCameraTarget _returnvalue_3) "NewEnumerator0")
    (Variables|Default|SetTarget%20Location (Math|Vector|MakeVector (.x _returnvalue) (.y _returnvalue) (.z (+ (Math|Vector|MakeVector 0.0 0.0 (.z (Transformation|GetActorLocation (Variables|/Game/99_MyContents/CAMERA/CameraController.CameraController_C|GetTopCamera _returnvalue_3)))) 2e+04)))) ; Location is Top Camera
    (else
      (Variables|Default|SetTarget%20Location (Math|Vector|MakeVector (.x _returnvalue_2) (.y _returnvalue_2) (.z (+ (Math|Vector|MakeVector 0.0 0.0 (.z (Transformation|GetActorLocation (Variables|/Game/99_MyContents/CAMERA/CameraController.CameraController_C|GetBottomCamera _returnvalue_3)))) 2e+04)))) ; Location is Bottom Camera
    ))
  (Transformation|SetActorLocationAndRotation (Variables|Default|GetTarget%20Location) (Variables|Default|GetTarget%20Rotation)))